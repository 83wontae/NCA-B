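; BP_MyActor is a practice actor whose static mesh slides back and forth along its relative X axis.
; Each Tick calls NewFunction, which, while IsPlay is set, steps the X position variable and flips IsMoveRight at either limit.
; BeginPlay prints a message and starts a looping timer by function name, whose OnUpdateTimer handler only prints text.
; Disconnected leftover nodes hold delayed step moves, a self-name print and unused operators.
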(event `self.ReceiveBeginPlay`
  (`KismetSystemLibrary.PrintString` "BeginPlay")
  (`KismetSystemLibrary.K2_SetTimer` null "OnUpdateTimer" 0.1 true))

(event `self.ReceiveTick`
  (params (DeltaSeconds :type "Float (single-precision)"))
  (`self.NewFunction`))

(fn `NewFunction`
  (if (`self.IsPlay`)
    (if (`self.IsMoveRight`)
      ;[1 1 1] X 방향으로 한번 움직인다
      (bind _output_get (set `self.X위치` (+ (`self.X위치`) 1.0)))
      (`SceneComponent.K2_SetRelativeLocation` (`self.StaticMesh`) (`KismetMathLibrary.MakeVector` _output_get) false false)
      (if (> (`self.X위치`) 100.0)
        (set `self.IsMoveRight` false))
      (else
        ;[1 1 1] X 반대 방향으로 한번 움직인다
        (bind _output_get_2 (set `self.X위치` (+ (`self.X위치`) -1.0)))
        (`SceneComponent.K2_SetRelativeLocation` (`self.StaticMesh`) (`KismetMathLibrary.MakeVector` _output_get_2) false false)
        (if (< (`self.X위치`) 0.0)
          (set `self.IsMoveRight` true))))))

(fn `OnUpdateTimer`
  (`KismetSystemLibrary.PrintString` "Timer"))

(fn `UserConstructionScript`)